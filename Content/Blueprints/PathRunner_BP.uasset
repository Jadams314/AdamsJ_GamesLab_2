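; Path runner actor that moves in straight lines through a list of point actors, looping back to the first after the last.
; While active, Tick moves it along a normalized direction at a set speed, without sweeping.
; Once it comes within range of the current point, it advances to the next one, recomputes its direction and snaps its rotation to face it.
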(event `self.ReceiveBeginPlay`
  (set `self.CurrentPoint` (`|GetArrayItem` (`self.PathList`)))
  (`self.SetMoveDirection`))

(event `self.ReceiveTick`
  (params (DeltaSeconds :type "Float (single-precision)"))
  (if (`self.IsActive`)
    (`self.MoveRunner` DeltaSeconds)
    (`self.CheckDistanceAndUpdate`)))

(fn `CheckDistanceAndUpdate`
  (if (< (`self.GetDistanceTo` (`self.CurrentPoint`)) (`self.PointWithinRange`))
    (`self.NextPathPoint`)
    (`self.SetMoveDirection`)))

(fn `MoveRunner`
  (params (DeltaSeconds :type "Float (double-precision)"))
  (`self.K2_SetActorLocation` self (+ (* DeltaSeconds (`self.MoveSpeed`) (`self.MoveDirection`)) (`self.K2_GetActorLocation` self)) false false))

(fn `NextPathPoint`
  (bind _pathlistindex (`self.PathListIndex`))
  (bind _pathlist (`self.PathList`))
  (bind _result (`/Engine/EditorBlueprintResources/StandardMacros.IncrementInt` _pathlistindex)
    (:`  `
      (if (== _result (`KismetArrayLibrary.Array_Length` _pathlist))
        (set `self.PathListIndex` 0))
      (set `self.CurrentPoint` (`|GetArrayItem` _pathlist _pathlistindex)))))

(fn `SetMoveDirection`
  (bind _returnvalue (`KismetMathLibrary.Normal` (- (`self.K2_GetActorLocation` (`self.CurrentPoint`)) (`self.K2_GetActorLocation`))))
  (set `self.MoveDirection` _returnvalue)
  (`self.K2_SetActorRotation` (`KismetMathLibrary.MakeRotFromX` _returnvalue)))

(fn `UserConstructionScript`)